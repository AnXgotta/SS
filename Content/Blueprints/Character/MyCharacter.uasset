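; Player character Blueprint that shows a debug inventory overlay while Tab is held.
; Pressing Tab creates a fresh debug widget showing the clothes' current weight against capacity, and releasing removes it from the viewport.
; Each entry in the clothes item map becomes a button labeled with item name and count.
; The helper returns each item widget's inner button, which is added to the list.
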(event Input|KeyboardEvents|Tab
  (:Pressed
    (bind _returnvalue (Utilities|Casting|CastToPlayerController (Pawn|GetController)))
    (CallFunction|CreateDebugUI _returnvalue))
  (:Released
    (CallFunction|RemoveDebugUI)))

(fn ConstructionScript)

(fn CreateDebugUI
  (params (PlayerController :type Player%20Controller%20Object%20Reference))
  (bind _playerclothes (Variables|Default|GetPlayerClothes))
  (bind _returnvalue (UserInterface|CreateWidget "/Game/UI/Widgets/BP_WidgetDebug_Inventory.BP_WidgetDebug_Inventory_C" PlayerController))
  (Variables|Default|SetUIWidgetDebug _returnvalue)
  (Variables|/Game/UI/Widgets/BP_WidgetDebug_Inventory.BP_WidgetDebug_Inventory_C|SetClothesWeightText (Variables|Default|GetUIWidgetDebug) (Utilities|String|Append (Utilities|String|Append (Utilities|String|ToString(Float) (Variables|/Script/SS.SSInventoryContainerBase|GetCurrentWeight _playerclothes)) " / ") (Utilities|String|ToString(Float) (Variables|/Script/SS.SSInventoryContainerBase|GetWeightCapacity _playerclothes))))
  (for _array_element (Variables|/Script/SS.SSInventoryContainerBase|GetItemMap _playerclothes)
    (bind _created_button (CallFunction|CreateButtonandSetText (Utilities|String|Append (Utilities|String|Append (.ItemName (Utilities|Struct|BreakContainerSlot _array_element)) " : ") (Utilities|String|ToString(Integer) (Utilities|Array|Length (.Items (Utilities|Struct|BreakContainerSlot _array_element)))))))
    (bind _aswidget (Utilities|Casting|CastToWidget _created_button))
    (Widget|Panel|AddChild (Variables|/Game/UI/Widgets/BP_WidgetDebug_Inventory.BP_WidgetDebug_Inventory_C|GetSB_Items (Variables|Default|GetUIWidgetDebug)) _aswidget))
  (UserInterface|Viewport|AddtoViewport (Variables|Default|GetUIWidgetDebug)))

(fn RemoveDebugUI
  (Class|UserWidget|RemovefromViewport (Variables|Default|GetUIWidgetDebug)))

(fn CreateButtonandSetText
  (params (Button%20Text :type String))
  (bind _returnvalue (UserInterface|CreateWidget "/Game/UI/Widgets/BP_Widget_Iten_Button.BP_Widget_Iten_Button_C" (Game|GetPlayerController 0)))
  (Rendering|Components|TextRender|SetText (Variables|/Game/UI/Widgets/BP_Widget_Iten_Button.BP_Widget_Iten_Button_C|GetButtonText _returnvalue) (Utilities|Text|ToText(String) Button%20Text))
  (return (Variables|/Game/UI/Widgets/BP_Widget_Iten_Button.BP_Widget_Iten_Button_C|GetButton_0 _returnvalue)))